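; Player spaceship that slides left and right to collect stars and avoid asteroids.
; While BP_GameMode is playing, axis input steps the ship along Y, bounded by the spline's world Y and its length.
; Overlaps destroy tagged stars or asteroids and tell the GameMode to increase score or decrease life.
; Delay-based tap-counting macros exist for a double-tap dash, which is unconnected and marked as not working.
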(event `InputAxis|HorizontalMovement`
  (params (AxisValue :type "Float (single-precision)"))
  (bind _spaceship (`self.Spaceship`))
  (bind _spaceship_2 (`self.Spaceship`))
  (bind (_returnvalue_x _returnvalue_y _returnvalue_z) (`KismetMathLibrary.BreakVector` (`SceneComponent.K2_GetComponentLocation` _spaceship)))
  (bind (_returnvalue_x_2 _returnvalue_y_2) (`KismetMathLibrary.BreakVector` (`SceneComponent.K2_GetComponentLocation` (`self.Spline`))))
  (bind (_returnvalue_x_3 _returnvalue_y_3 _returnvalue_z_2) (`KismetMathLibrary.BreakVector` (`SceneComponent.K2_GetComponentLocation` _spaceship_2)))
  (bind _returnvalue (- _returnvalue_y (`self.MovementSpeed`)))
  (bind _returnvalue_2 (+ _returnvalue_y_3 (`self.MovementSpeed`)))
  ;[1 1 1] Checks if Game Over
  (bind _asbp_game_mode (cast `/Game/Blueprints/BP_GameMode` (`GameplayStatics.GetGameMode`)))
  (if (`/Game/Blueprints/BP_GameMode.IsPlaying` _asbp_game_mode)
    ;[1 1 1] SpaceshipMovement
    (if (< AxisValue 0.0)
      (if (not (< _returnvalue _returnvalue_y_2))
        ;[1 1 1] Left
        (`SceneComponent.K2_SetWorldLocation` _spaceship (`KismetMathLibrary.MakeVector` _returnvalue_x _returnvalue _returnvalue_z) false false))
      (elif (> AxisValue 0.0)
        (if (not (> _returnvalue_2 (`SplineComponent.GetSplineLength` (`self.Spline`))))
          ;[1 1 1] Right
          (`SceneComponent.K2_SetWorldLocation` _spaceship_2 (`KismetMathLibrary.MakeVector` _returnvalue_x_3 _returnvalue_2 _returnvalue_z_2) false false))))))

(event `Key|D`
  (params (Key :type "Key Structure"))
  ;[1 1 1] *Doesn't Work* Double tap either direction to dash in that direction
)

(event `Key|A`
  (params (Key :type "Key Structure"))
  ;[1 1 1] *Doesn't Work* Double tap either direction to dash in that direction
)

(event `self.Collision.OnComponentBeginOverlap`
  (params (OverlappedComponent :type "PrimitiveComponent Object Reference") (OtherActor :type "Actor Object Reference") (OtherComp :type "PrimitiveComponent Object Reference") (OtherBodyIndex :type Integer) (bFromSweep :type Boolean) (SweepResult :type "HitResult Structure (by ref)"))
  ;[1 1 1] Checks what collided with Spaceship
  (if (`self.ActorHasTag` OtherActor "star")
    ;[1 1 1] Destroy's actor and alters score depending on what collided
    (`self.K2_DestroyActor` OtherActor)
    (bind _asbp_game_mode (cast `/Game/Blueprints/BP_GameMode` (`GameplayStatics.GetGameMode`)))
    (`/Game/Blueprints/BP_GameMode.IncreaseScore` _asbp_game_mode)
    (elif (`self.ActorHasTag` OtherActor "asteroid")
      (`self.K2_DestroyActor` OtherActor)
      (bind _asbp_game_mode_2 (cast `/Game/Blueprints/BP_GameMode` (`GameplayStatics.GetGameMode`)))
      (`/Game/Blueprints/BP_GameMode.DecreaseLife` _asbp_game_mode_2))))

(fn `UserConstructionScript`)