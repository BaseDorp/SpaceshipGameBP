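; Spawner actor that periodically drops random asteroids and stars into the level while BP_GameMode reports IsPlaying.
; BeginPlay starts two events that each re-arm their own looping timer, using separate asteroid and star spawn rates.
; Each spawn picks a random Y offset around the spawner, with asteroids chosen from four classes.
; All branches share one SetLifeSpan node targeting the last spawned star, so asteroids receive no lifespan here.
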(event `StartSpawningAsteroid`
  (bind (_returnvalue_x _returnvalue_y _returnvalue_z) (`KismetMathLibrary.BreakVector` (`self.K2_GetActorLocation`)))
  (bind _returnvalue (`KismetMathLibrary.MakeTransform` (`KismetMathLibrary.MakeVector` _returnvalue_x (`KismetMathLibrary.RandomFloatInRange` (- _returnvalue_y 500.0) (+ _returnvalue_y 500.0)) _returnvalue_z) (`KismetMathLibrary.RandomRotator` false)))
  ;[1 1 1] Starts timer for spawning actors
  (`KismetSystemLibrary.K2_SetTimerDelegate` (delegate `StartSpawningAsteroid`) (`self.AstroidSpawnRate`) true)
  (bind _asbp_game_mode (cast `/Game/Blueprints/BP_GameMode` (`GameplayStatics.GetGameMode`)))
  (if (`/Game/Blueprints/BP_GameMode.IsPlaying` _asbp_game_mode)
    (switch `int` (`KismetMathLibrary.RandomIntegerInRange` 0 3)
      (:`0`
        (bind _returnvalue_2 (`|SpawnActorFromClass` "/Game/Blueprints/BP_Asteroid.BP_Asteroid_C" _returnvalue "Undefined" "OverrideRootScale" null null))
        (`/Engine/EditorBlueprintResources/StandardMacros.IsValid` _returnvalue_2
          (:`Is Valid`
            _)))
      (:`1`
        (bind _returnvalue_3 (`|SpawnActorFromClass` "/Game/Blueprints/BP_Asteroid2.BP_Asteroid2_C" _returnvalue "Undefined" "OverrideRootScale" null null))
        (`/Engine/EditorBlueprintResources/StandardMacros.IsValid` _returnvalue_3
          (:`Is Valid`
            _)))
      (:`2`
        (bind _returnvalue_4 (`|SpawnActorFromClass` "/Game/Blueprints/BP_Asteroid3.BP_Asteroid3_C" _returnvalue "Undefined" "OverrideRootScale" null null))
        (`/Engine/EditorBlueprintResources/StandardMacros.IsValid` _returnvalue_4
          (:`Is Valid`
            _)))
      (:`3`
        (bind _returnvalue_5 (`|SpawnActorFromClass` "/Game/Blueprints/BP_Asteroid4.BP_Asteroid4_C" _returnvalue "Undefined" "OverrideRootScale" null null))
        (`/Engine/EditorBlueprintResources/StandardMacros.IsValid` _returnvalue_5
          (:`Is Valid`
            _))))
    ;[1 1 1] Destroys the Actor after a certain amount of time
    (`self.SetLifeSpan` (stale `StartSpawningStar` _returnvalue) 4.0 :!label _label)))

(event `self.ReceiveBeginPlay`
  (`self.StartSpawningStar`)
  (`self.StartSpawningAsteroid`))

(event `StartSpawningStar`
  (bind (_returnvalue_x _returnvalue_y _returnvalue_z) (`KismetMathLibrary.BreakVector` (`self.K2_GetActorLocation`)))
  ;[1 1 1] Starts timer for spawning actors
  (`KismetSystemLibrary.K2_SetTimerDelegate` (delegate `StartSpawningStar`) (`self.StarSpawnRate`) true)
  (bind _asbp_game_mode (cast `/Game/Blueprints/BP_GameMode` (`GameplayStatics.GetGameMode`)))
  (if (`/Game/Blueprints/BP_GameMode.IsPlaying` _asbp_game_mode)
    (bind _returnvalue (`|SpawnActorFromClass` "/Game/Blueprints/BP_Star.BP_Star_C" (`KismetMathLibrary.MakeTransform` (`KismetMathLibrary.MakeVector` _returnvalue_x (`KismetMathLibrary.RandomFloatInRange` (- _returnvalue_y 500.0) (+ _returnvalue_y 500.0)) _returnvalue_z) (`KismetMathLibrary.RandomRotator` false)) "Undefined" "OverrideRootScale" null null))
    (goto _label)))

(fn `UserConstructionScript`)