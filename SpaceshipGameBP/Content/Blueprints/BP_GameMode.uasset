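; BP_GameMode is a game mode that tracks score, lives and whether play is active.
; DecreaseLife and IncreaseScore events change the counters only while IsPlaying is true, and losing the last life clears IsPlaying as the game-over state.
; On BeginPlay it creates the BP_UI widget, stores it and adds it to the viewport.
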(event `DecreaseLife`
  (bind _lives (`self.Lives`))
  ;[1 1 1] Remove Life
  (if (`self.IsPlaying`)
    (set `self.Lives` (- _lives 1))
    ;[1 1 1] Game Over State
    (if (<= _lives 0)
      (set `self.IsPlaying` false))))

(event `IncreaseScore`
  ;[1 1 1] Increase Score
  (if (`self.IsPlaying`)
    (set `self.Score` (+ (`self.Score`) 1))))

(event `self.ReceiveBeginPlay`
  ;[1 1 1] Puts UI on screen
  (bind _returnvalue (`|CreateWidget` "/Game/Blueprints/BP_UI.BP_UI_C"))
  (bind _output_get (set `self.UI` _returnvalue))
  (`UserWidget.AddToViewport` _output_get 0))

(fn `UserConstructionScript`)